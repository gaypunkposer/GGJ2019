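; VR toaster prop that makes toast for an objective and kills the player if a fork is inserted.
; The Load button lowers a lerped mesh, and Tick polls HitDetect overlaps for forks or released toast.
; A fork triggers sparks, haptics and VR_Pawn death, while toast attaches with collision off.
; The Toast button waits, launches the bread upward, raises the mesh and updates the objective once if CanScore is set.
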(event `self.ReceiveBeginPlay`
  (bind _outactors (`GameplayStatics.GetAllActorsOfClass` "/Game/VR_Pawn.VR_Pawn_C"))
  (set `self.VR_PawnIsnt` (`|GetArrayItem` _outactors))
  (bind _outactors_2 (`GameplayStatics.GetAllActorsOfClass` "/Game/GripProps/WatchStateMachine.WatchStateMachine_C"))
  (bind _aswatch_state_machine (cast `/Game/GripProps/WatchStateMachine` (`|GetArrayItem` _outactors_2)))
  (set `self.Watch` _aswatch_state_machine))

(event `self.Load.OnButtonStateChanged`
  (params (ButtonState :type Boolean) (InteractingActor :type "Actor Object Reference") (InteractingComponent :type "PrimitiveComponent Object Reference"))
  (bind _asvr_pawn (cast `/Game/VR_Pawn` InteractingActor))
  (`/Game/VR_Pawn.Haptic Feedback` _asvr_pawn 5.0 0.05 (`KismetStringLibrary.Contains` (`KismetSystemLibrary.GetDisplayName` InteractingComponent) "Left"))
  (set `self.Lowered` ButtonState))

(event `self.ReceiveTick`
  (params (DeltaSeconds :type "Float (single-precision)"))
  (bind _vr_pawnisnt (`self.VR_PawnIsnt`))
  (bind _staticmesh6 (`self.StaticMesh6`))
  (bind _relativelocation (`SceneComponent.RelativeLocation` _staticmesh6))
  (`|ExecutionSequence`
    (:`then_0`
      (if (`self.Lowered`)
        (`SceneComponent.K2_SetRelativeLocation` _staticmesh6 (`KismetMathLibrary.VLerp` _relativelocation (0.0 0.0 -100.0) 0.5) false false)
        (else
          (`SceneComponent.K2_SetRelativeLocation` _staticmesh6 (`KismetMathLibrary.VLerp` _relativelocation (0.0 0.0 0.0) 0.5) false false))))
    (:`then_1`
      (for _array_element (`PrimitiveComponent.GetOverlappingActors` (`self.HitDetect`) "/Game/VR_GripObject.VR_GripObject_C")
        (`|ExecutionSequence`
          (:`then_0`
            (if (== (`GameplayStatics.GetObjectClass` _array_element) "/Game/GripProps/ForkBP.ForkBP_C")
              (if (not (`self.Electricuted`))
                (set `self.Electricuted` true)
                (`ActorComponent.Activate` (`self.P_Sparks`) true)
                (if (`KismetSystemLibrary.IsValid` _vr_pawnisnt)
                  (`/Game/VR_Pawn.Haptic Feedback` _vr_pawnisnt 1000.0 5.0 true)
                  (`/Game/VR_Pawn.Haptic Feedback` _vr_pawnisnt 1000.0 5.0 false)
                  (`ActorComponent.Activate` (`self.zap`) false)
                  (`/Game/VR_Pawn.Die` _vr_pawnisnt "Home is where you, wait did you just put a fork in the toaster? Dude are you alright?")))))
          (:`then_1`
            (if (== (`GameplayStatics.GetObjectClass` _array_element) "/Game/GripProps/ToastBP.ToastBP_C")
              (bind (_holdingcontroller _bisheld) (message `VRGripInterface.IsHeld` _array_element))
              (bind _returnvalue (not _bisheld))
              (`KismetSystemLibrary.PrintString` "Hello" _returnvalue)
              (if (and (`self.Lowered`) _returnvalue)
                (set `self.RawToastIn` true)
                (bind _astoast_bp (cast `/Game/GripProps/ToastBP` _array_element))
                (`self.ToasterActive` _astoast_bp)))))))))

(event `self.SetOutline`
  (params (Enabled :type Boolean))
  (if (and Enabled false)
    (`PrimitiveComponent.SetRenderCustomDepth` (`self.Load`) true)
    (`PrimitiveComponent.SetRenderCustomDepth` (`self.Toast`) true)
    (else
      (`PrimitiveComponent.SetRenderCustomDepth` (`self.Toast`) false)
      (`PrimitiveComponent.SetRenderCustomDepth` (`self.Load`) false))))

(event `self.Toast.OnButtonBeginInteraction`
  (params (InteractingActor :type "Actor Object Reference") (InteractingComponent :type "PrimitiveComponent Object Reference"))
  (bind _returnvalue (`SceneComponent.GetUpVector` (`self.StaticMesh`)))
  (bind _asvr_pawn (cast `/Game/VR_Pawn` InteractingActor))
  (`/Game/VR_Pawn.Haptic Feedback` _asvr_pawn 5.0 0.05 (`KismetStringLibrary.Contains` (`KismetSystemLibrary.GetDisplayName` InteractingComponent) "Left"))
  (if (`self.RawToastIn`)
    (`KismetSystemLibrary.Delay` 5.0)
    (`self.K2_DetachFromActor` (stale `self.ReceiveTick` _astoast_bp) "KeepWorld" "KeepWorld" "KeepRelative")
    (bind _staticmesh (`/Game/VR_GripObject.StaticMesh` (stale `self.ReceiveTick` _astoast_bp)))
    (`SceneComponent.K2_AddWorldOffset` _staticmesh (* _returnvalue 100.0) false true)
    (`PrimitiveComponent.SetCollisionEnabled` _staticmesh "PhysicsOnly")
    (`PrimitiveComponent.AddForce` _staticmesh (* _returnvalue 50000.0) "None" true)
    (`KismetSystemLibrary.Delay` 0.025)
    (set `self.Lowered` false)
    (if (`self.CanScore`)
      (`/Game/VR_Pawn.UpdateObj` (`self.VR_PawnIsnt`) 3)
      (set `self.CanScore` false))))

(fn `ToasterActive`
  (params (MuhBread :type "/Game/GripProps/ToastBP Object Reference"))
  (`self.K2_AttachToActor` MuhBread self "None" "KeepRelative" "KeepRelative" "KeepWorld" true)
  (`ActorComponent.Activate` (`self.Beep`) false)
  (`SceneComponent.K2_SetWorldLocationAndRotation` (`/Game/VR_GripObject.StaticMesh` MuhBread) (`self.K2_GetActorLocation`) (`self.K2_GetActorRotation`) false true)
  (`self.K2_AddActorLocalOffset` MuhBread (35.0 0.0 150.0) false true)
  (`PrimitiveComponent.SetCollisionEnabled` (`/Game/VR_GripObject.StaticMesh` MuhBread) "NoCollision")
  (set `self.RawToastIn` true))

(fn `UserConstructionScript`
  (`parent.UserConstructionScript`))