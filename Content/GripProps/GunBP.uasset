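; GunBP is a VR grip prop, a brush gun that checks on use whether it is aimed at the player's head.
; BeginPlay caches the first VR_Pawn in the level.
; OnUsed fires the explosion effect and line-traces along its right vector against only that pawn's HeadCollision, printing a debug message on a hit and leaving the trace drawn.
; SetOutline toggles custom depth on the gun mesh for highlighting.
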(event `self.OnUsed`
  (bind _p_explosion (`self.P_Explosion`))
  (bind _returnvalue (`SceneComponent.K2_GetComponentLocation` _p_explosion))
  (bind _returnvalue_2 (`SceneComponent.GetRightVector` _p_explosion))
  (`ActorComponent.Activate` (`self.P_Explosion`) true)
  (bind (_hitlocation _hitnormal _bonename _outhit _returnvalue_3) (`PrimitiveComponent.K2_LineTraceComponent` (`/Game/VR_Pawn.Head Collision` (`self.VR_PawnIsnt`)) (+ _returnvalue (* _returnvalue_2 0.0)) (+ _returnvalue (* _returnvalue_2 1000.0)) true true true))
  (if _returnvalue_3
    (`KismetSystemLibrary.PrintString` "FACE BRUSHED")))

(event `self.SetOutline`
  (params (Enabled :type Boolean))
  (`PrimitiveComponent.SetRenderCustomDepth` (`self.brushgun1_low`) Enabled))

(event `self.ReceiveBeginPlay`
  (bind _outactors (`GameplayStatics.GetAllActorsOfClass` "/Game/VR_Pawn.VR_Pawn_C"))
  (bind _asvr_pawn (cast `/Game/VR_Pawn` (`|GetArrayItem` _outactors)))
  (set `self.VR_PawnIsnt` _asvr_pawn))

(fn `UserConstructionScript`
  (`parent.UserConstructionScript`))