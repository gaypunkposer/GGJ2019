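; Grippable VR toothbrush prop that advances a player objective once when used while aimed at the player's head.
; It caches the VR pawn at start and tracks the gripping controller, whose display name picks the hand for haptic feedback.
; On use, a particle effect plays for a second while a short, debug-drawn trace from it tests only the pawn's head collision.
; A hit updates the objective after that delay.
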(event `self.ReceiveBeginPlay`
  (bind _outactors (`GameplayStatics.GetAllActorsOfClass` "/Game/VR_Pawn.VR_Pawn_C"))
  (bind _asvr_pawn (cast `/Game/VR_Pawn` (`|GetArrayItem` _outactors)))
  (set `self.VR_PawnIsnt` _asvr_pawn))

(event `VRGripInterface.OnGrip`
  (params (GrippingController :type "GripMotionControllerComponent Object Reference") (GripInformation :type "BPActorGripInformation Structure (by ref)"))
  (set `self.GrabbedHand` GrippingController))

(event `self.OnGripRelease`
  (params (ReleasingController :type "GripMotionControllerComponent Object Reference") (GripInformation :type "BPActorGripInformation Structure (by ref)") (bWasSocketed :type Boolean))
  (set `self.GrabbedHand` null))

(event `self.OnUsed`
  (bind _p_steam_lit (`self.P_Steam_Lit`))
  (bind _returnvalue (`SceneComponent.K2_GetComponentLocation` _p_steam_lit))
  (`/Game/VR_Pawn.Haptic Feedback` (`self.VR_PawnIsnt`) 25.0 0.05 (`KismetStringLibrary.Contains` (`KismetSystemLibrary.GetDisplayName` (`self.GrabbedHand`)) "Left"))
  (`ActorComponent.Activate` _p_steam_lit false)
  (bind (_hitlocation _hitnormal _bonename _outhit _returnvalue_2) (`PrimitiveComponent.K2_LineTraceComponent` (`/Game/VR_Pawn.Head Collision` (`self.VR_PawnIsnt`)) _returnvalue (+ _returnvalue (* (`SceneComponent.GetForwardVector` _p_steam_lit) 50.0)) true true true))
  (`KismetSystemLibrary.Delay` 1.0)
  (`ActorComponent.Deactivate` (`self.P_Steam_Lit`))
  (if _returnvalue_2
    (if (`self.CanScore`)
      (`/Game/VR_Pawn.UpdateObj` (`self.VR_PawnIsnt`) 1)
      (set `self.CanScore` false))))

(fn `UserConstructionScript`
  (`parent.UserConstructionScript`))